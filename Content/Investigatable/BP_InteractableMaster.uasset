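; Base actor for investigatable objects, hidden at start if investigate-locked, which registers with the ThirdPersonCharacter on proximity overlap.
; A looping timer pulses its indicator while overlapped, and leaving ends the investigation.
; DT_InvestigatableObjectInfo rows, keyed by ObjectID, supply name and description, or new information once revealed.
; UnlockInteractionsF flags linked objects' new information, clears equip locks on equipables and unhides unequipped or non-equipable ones.
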(event `self.ReceiveBeginPlay`
  ;[1 1 1] Begin Play - Set investigate locks
  (if (`self.InvestigateLocked`)
    (`self.SetActorHiddenInGame` true)))

(event `PulsateIndicator`
  ;[1 1 1] Pulsate Indicator
  (bind _isa (`/Engine/EditorBlueprintResources/StandardMacros.FlipFlop` :!label _label)
    (:`A`
      (bind (_direction _scale) (`Timeline|PulsateIndicator_Timeline` :!via `PlayFromStart` :!label _label_2)
        (:`Update`
          (`SceneComponent.SetRelativeScale3D` (`self.Indicator`) (`KismetMathLibrary.MakeVector` _scale _scale _scale))
          (`KismetSystemLibrary.Delay` 0.4)
          (if _isa
            (goto _label)))))
    (:`B`
      (goto _label_2 :!via `ReverseFromEnd`))))

(event `self.ProximityCollision.OnComponentBeginOverlap`
  (params (OverlappedComponent :type "PrimitiveComponent Object Reference") (OtherActor :type "Actor Object Reference") (OtherComp :type "PrimitiveComponent Object Reference") (OtherBodyIndex :type Integer) (bFromSweep :type Boolean) (SweepResult :type "HitResult Structure (by ref)"))
  ;[1 1 1] Overlap Indicator & set current investigatable object reference
  (bind _asthird_person_character (cast `/Game/PlayerCharacter/ThirdPersonCharacter` OtherActor))
  (set `/Game/PlayerCharacter/ThirdPersonCharacter.InvestigatableObject` self _asthird_person_character)
  (if (not (`self.IsOverlapping`))
    (set `self.IsOverlapping` true)
    (bind _returnvalue (`KismetSystemLibrary.K2_SetTimer` null "PulsateIndicator" 1.0 true -1.0))))

(event `self.ProximityCollision.OnComponentEndOverlap`
  (params (OverlappedComponent :type "PrimitiveComponent Object Reference") (OtherActor :type "Actor Object Reference") (OtherComp :type "PrimitiveComponent Object Reference") (OtherBodyIndex :type Integer))
  ;[1 1 1] Overlap Indicator & set current investigatable object reference
  (bind _asthird_person_character (cast `/Game/PlayerCharacter/ThirdPersonCharacter` OtherActor))
  (`/Game/PlayerCharacter/ThirdPersonCharacter.End Investigation` _asthird_person_character)
  (set `self.IsOverlapping` false)
  (`KismetSystemLibrary.K2_ClearAndInvalidateTimerHandle` (stale `self.ProximityCollision.OnComponentBeginOverlap` _returnvalue)))

(fn `CurrentDialogueF`
  (returns (CurrentObjectDescription :type Text) (CurrentObjectName :type Text))
  (bind _returnvalue (`|GetDataTableRow` "/Game/Investigatable/DT_InvestigatableObjectInfo.DT_InvestigatableObjectInfo" (`self.ObjectID`))
    (:`then`
      (if (`self.ShowNewInformation`)
        (bind (_objectname _objectdescription _newinformation) (break `/Game/Investigatable/F_InvestigatableObjectStruct` _returnvalue))
        (if (`KismetTextLibrary.TextIsEmpty` _newinformation)
          _
          (else
            (return _newinformation _objectname))))
      (return _objectdescription _objectname))))

(fn `UnlockInteractionsF`
  (for _array_element (`self.UnlocksObjects`)
    (set `/Game/Investigatable/BP_InteractableMaster.ShowNewInformation` true _array_element)
    (bind _returnvalue (`|GetDataTableRow` "/Game/Investigatable/DT_InvestigatableObjectInfo.DT_InvestigatableObjectInfo" (`/Game/Investigatable/BP_InteractableMaster.ObjectID` _array_element))
      (:`then`
        (if (`.Equipable_10_BD14E3BD4162D3D9B80F34839F201211` (break `/Game/Investigatable/F_InvestigatableObjectStruct` _returnvalue))
          (set `/Game/Investigatable/BP_InteractableMaster.EquipLocked` false _array_element)
          (if (not (`/Game/Investigatable/BP_InteractableMaster.Equipped` _array_element))
            (`self.SetActorHiddenInGame` _array_element false :!label _label))
          (else
            (goto _label)))))))

(fn `UserConstructionScript`)